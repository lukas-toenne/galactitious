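; Grabbable galaxy rim ring actor that gives visual feedback when focused or grabbed.
; The construction script approximates the ring's collision with capsules laid end to end as a polygon, sized from Radius, Segments and Thickness.
; At BeginPlay it creates a dynamic MI_Grabbable material on the ring.
; BP_GalaxyGrabTarget focus and grab events drive that material's focus state, grab state and grab position.
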(event `self.ReceiveBeginPlay`
  (bind _returnvalue (`PrimitiveComponent.CreateDynamicMaterialInstance` (`self.0_GalaxyRing`) 0 "/Game/Materials/MI_Grabbable.MI_Grabbable" "None"))
  (set `self.Material` _returnvalue))

(event `self.ReceiveTick`
  (params (DeltaSeconds :type "Float (single-precision)")))

(event `self.BP_GalaxyGrabTarget.OnBeginGrab`
  (params (Grabbable :type "UxtGrabTargetComponent Object Reference") (GrabPointer :type "UxtGrabPointerData Structure"))
  (`self.UpdateMaterialGrab` true GrabPointer))

(event `self.BP_GalaxyGrabTarget.OnEnterFocus`
  (params (Pointer :type "UxtNearPointerComponent Object Reference"))
  (`self.UpdateMaterialFocus` true))

(event `self.BP_GalaxyGrabTarget.OnUpdateGrab`
  (params (Grabbable :type "UxtGrabTargetComponent Object Reference") (GrabPointer :type "UxtGrabPointerData Structure"))
  (`self.UpdateMaterialGrab` true GrabPointer))

(event `self.BP_GalaxyGrabTarget.OnUpdateFocus`
  (params (Pointer :type "UxtNearPointerComponent Object Reference")))

(event `self.BP_GalaxyGrabTarget.OnEndGrab`
  (params (Grabbable :type "UxtGrabTargetComponent Object Reference") (GrabPointer :type "UxtGrabPointerData Structure"))
  (`self.UpdateMaterialGrab` false GrabPointer))

(event `self.BP_GalaxyGrabTarget.OnExitFocus`
  (params (Pointer :type "UxtNearPointerComponent Object Reference"))
  (`self.UpdateMaterialFocus` false))

(fn `UpdateMaterialFocus`
  (params (IsFocused :type Boolean))
  (`MaterialInstanceDynamic.SetScalarParameterValue` (`self.Material`) "IsFocused" (`KismetMathLibrary.Conv_BoolToDouble` IsFocused)))

(fn `UpdateMaterialGrab`
  (params (IsGrabbed :type Boolean) (GrabPointerData :type "UxtGrabPointerData Structure (by ref)"))
  (bind _material (`self.Material`))
  (`MaterialInstanceDynamic.SetScalarParameterValue` _material "IsGrabbed" (`KismetMathLibrary.Conv_BoolToDouble` IsGrabbed))
  (`MaterialInstanceDynamic.SetVectorParameterValue` _material "GrabPosition" (`KismetMathLibrary.Conv_VectorToLinearColor` (`UxtGrabPointerDataFunctionLibrary.GetGrabLocation` (`self.GetTransform`) GrabPointerData))))

(fn `UserConstructionScript`
  (bind _segments (`self.Segments`))
  (bind _radius (`self.Radius`))
  (bind _returnvalue (* (`self.Thickness`) 0.5))
  (bind _returnvalue_2 (/ 360.0 (`KismetMathLibrary.Conv_IntToDouble` _segments)))
  (bind _returnvalue_3 (* _returnvalue_2 0.5))
  (bind _returnvalue_4 (* _radius (`KismetMathLibrary.DegCos` _returnvalue_3)))
  (for _index (range _segments)
    (bind _returnvalue_5 (* _index _returnvalue_2))
    (bind _returnvalue_6 (`AddComponent|NODE_AddCapsuleComponent-0` :`RelativeTransform` (`KismetMathLibrary.MakeTransform` (`KismetMathLibrary.MakeVector` (* _returnvalue_4 (`KismetMathLibrary.DegCos` _returnvalue_5)) (* _returnvalue_4 (`KismetMathLibrary.DegSin` _returnvalue_5))) (`KismetMathLibrary.MakeRotator` 90.0 0.0 _returnvalue_5))))
    (`CapsuleComponent.SetCapsuleSize` _returnvalue_6 _returnvalue (+ _returnvalue (* _radius (`KismetMathLibrary.DegSin` _returnvalue_3))) false)))