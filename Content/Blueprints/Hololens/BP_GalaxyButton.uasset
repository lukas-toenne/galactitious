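; BP_GalaxyButton is a HoloLens pressable button that gives visual and audio feedback on focus, press and release.
; On BeginPlay it creates a dynamic material on MovingVisuals and caches its Base Color.
; PressableButton focus events double that color when hover starts and restore it when the last focus ends.
; Press and release each play their own 2D sound, with no other action attached in this Blueprint.
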(event `self.ReceiveBeginPlay`
  (bind _movingvisuals (`self.MovingVisuals`))
  ;[1 1 1] Create a dynamic material instance so we can update it to reflect button state
  (bind _returnvalue (`PrimitiveComponent.CreateDynamicMaterialInstance` _movingvisuals 0 (`PrimitiveComponent.GetMaterial` _movingvisuals 0) "None"))
  ;[1 1 1] Store initial base color
  (bind _returnvalue_2 (`MaterialInstanceDynamic.K2_GetVectorParameterValue` _returnvalue "Base Color"))
  (set `self.BaseColor` _returnvalue_2))

(event `self.PressableButton.OnButtonPressed`
  (params (Button :type "UxtPressableButtonComponent Object Reference"))
  ;[1 1 1] Play sound on press
  (`GameplayStatics.PlaySound2D` (`self.PressedSound`) 1.0 1.0 0.0 null null))

(event `self.PressableButton.OnBeginFocus`
  (params (Button :type "UxtPressableButtonComponent Object Reference") (Pointer :type "Object Object Reference") (bWasAlreadyFocused :type Boolean))
  (if (not bWasAlreadyFocused)
    ;[1 1 1] Lighten base color on hover start
    (`MeshComponent.SetVectorParameterValueOnMaterials` (`self.MovingVisuals`) "Base Color" (`KismetMathLibrary.Conv_LinearColorToVector` (* (`self.BaseColor`) 2.0)))))

(event `self.PressableButton.OnButtonReleased`
  (params (Button :type "UxtPressableButtonComponent Object Reference"))
  ;[1 1 1] Play sound on release
  (`GameplayStatics.PlaySound2D` (`self.ReleasedSound`) 1.0 1.0 0.0 null null))

(event `self.PressableButton.OnEndFocus`
  (params (Button :type "UxtPressableButtonComponent Object Reference") (Pointer :type "Object Object Reference") (bIsStillFocused :type Boolean))
  (if (not bIsStillFocused)
    ;[1 1 1] Re-set original base color on hover end
    (`MeshComponent.SetVectorParameterValueOnMaterials` (`self.MovingVisuals`) "Base Color" (`KismetMathLibrary.Conv_LinearColorToVector` (`self.BaseColor`)))))

(fn `UserConstructionScript`)