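; BP_GalaxyManipulator is a grabbable HoloLens actor that gives visual feedback for hand focus and grab interaction on its mesh.
; At BeginPlay it creates a dynamic instance of MI_Grabbable on the mesh.
; BP_GalaxyGrabTarget events drive that material's focus and grab flags, and pass the grab location to the shader when a grab begins, updates or ends.
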(event `self.ReceiveBeginPlay`
  (bind _returnvalue (`PrimitiveComponent.CreateDynamicMaterialInstance` (`self.Mesh`) 0 "/Game/Materials/Hololens/MI_Grabbable.MI_Grabbable" "None"))
  (set `self.Material` _returnvalue))

(event `self.BP_GalaxyGrabTarget.OnBeginGrab`
  (params (GrabPointer :type " Structure"))
  (`self.UpdateMaterialGrab` true GrabPointer))

(event `self.BP_GalaxyGrabTarget.OnEnterFocus`
  (`self.UpdateMaterialFocus` true))

(event `self.BP_GalaxyGrabTarget.OnUpdateGrab`
  (params (GrabPointer :type " Structure"))
  (`self.UpdateMaterialGrab` true GrabPointer))

(event `self.BP_GalaxyGrabTarget.OnUpdateFocus`)

(event `self.BP_GalaxyGrabTarget.OnEndGrab`
  (params (GrabPointer :type " Structure"))
  (`self.UpdateMaterialGrab` false GrabPointer))

(event `self.BP_GalaxyGrabTarget.OnExitFocus`
  (`self.UpdateMaterialFocus` false))

(fn `UpdateMaterialFocus`
  (params (IsFocused :type Boolean))
  (`MaterialInstanceDynamic.SetScalarParameterValue` (`self.Material`) "IsFocused" (`KismetMathLibrary.Conv_BoolToDouble` IsFocused)))

(fn `UpdateMaterialGrab`
  (params (IsGrabbed :type Boolean) (GrabPointerData :type " Structure (by ref)"))
  (bind _material (`self.Material`))
  (`MaterialInstanceDynamic.SetScalarParameterValue` _material "IsGrabbed" (`KismetMathLibrary.Conv_BoolToDouble` IsGrabbed))
  (`MaterialInstanceDynamic.SetVectorParameterValue` _material "GrabPosition" (`KismetMathLibrary.Conv_VectorToLinearColor` (`self.GetGrabLocation` (`self.GetTransform`) GrabPointerData))))

(fn `UserConstructionScript`)