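; BP_HololensGalaxy is a HoloLens galaxy actor that can be moved and rotated by grabbing.
; Hub and rim child BP_GalaxyManipulator actors expose grab targets, whose events are bound on BeginPlay.
; Rim grabs yaw the Galaxy component in parent space, aligning the local grab point with the pointer target while keeping Z up.
; Hub grabs cache the actor transform, then offset its location from it.
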(event `self.ReceiveBeginPlay`
  (bind _bp_galaxygrabtarget (`self.GetGrabTarget` (`self.HubChildActor`)))
  ;[1 1 1] Bind to Rim Update
  (add `UxtGrabTargetComponent.OnUpdateGrab` (`self.GetGrabTarget` (`self.RimChildActor`)) (delegate `OnUpdateGrab_Event_0`))
  ;[1 1 1] Bind to Hub Update
  (add `UxtGrabTargetComponent.OnBeginGrab` _bp_galaxygrabtarget (delegate `OnBeginGrab_Event_1`))
  (add `UxtGrabTargetComponent.OnUpdateGrab` _bp_galaxygrabtarget (delegate `OnUpdateGrab_Event_1`)))

(event `OnBeginGrab_Event_1`
  (params (Grabbable :type "UxtGrabTargetComponent Object Reference") (GrabPointer :type "UxtGrabPointerData Structure"))
  ;[1 1 1] Bind to Hub Update
  (set `self.InitialTransform` (`self.GetTransform`)))

(event `OnUpdateGrab_Event_0`
  (params (Grabbable :type "UxtGrabTargetComponent Object Reference") (GrabPointer :type "UxtGrabPointerData Structure"))
  ;[1 1 1] Bind to Rim Update
  (`self.RotateGalaxy` GrabPointer))

(event `OnUpdateGrab_Event_1`
  (params (Grabbable :type "UxtGrabTargetComponent Object Reference") (GrabPointer :type "UxtGrabPointerData Structure"))
  ;[1 1 1] Bind to Hub Update
  (`self.MoveRoot` GrabPointer))

(fn `GetGrabTarget`
  (params (ChildActor :type "ChildActorComponent Object Reference"))
  (returns (BP_GalaxyGrabTarget :type "/Game/Blueprints/Hololens/BP_GalaxyGrabTarget Object Reference"))
  (bind _asbp_galaxy_manipulator (cast `/Game/Blueprints/Hololens/BP_GalaxyManipulator` (`ChildActorComponent.ChildActor` ChildActor)))
  (return (`/Game/Blueprints/Hololens/BP_GalaxyManipulator.BP_GalaxyGrabTarget` _asbp_galaxy_manipulator)))

(fn `GetParentTransform`
  (params (SceneComponent :type "SceneComponent Object Reference"))
  (returns (Transform :type "Transform Structure"))
  (bind _returnvalue (`SceneComponent.GetAttachParent` SceneComponent))
  (`/Engine/EditorBlueprintResources/StandardMacros.IsValid` _returnvalue
    (:`Is Valid`
      (return (`SceneComponent.K2_GetComponentToWorld` _returnvalue)))
    (:`Is Not Valid`
      (return (`KismetMathLibrary.MakeTransform` (0.0 0.0 0.0))))))

(fn `MoveRoot`
  (params (GrabPointer :type "UxtGrabPointerData Structure"))
  (bind _initialtransform (`self.InitialTransform`))
  (`self.K2_SetActorLocation` (+ (.location _initialtransform) (`UxtGrabPointerDataFunctionLibrary.GetLocationOffset` _initialtransform GrabPointer))))

(fn `RotateGalaxy`
  (params (GrabPointer :type "UxtGrabPointerData Structure (by ref)"))
  (bind _returnvalue (`KismetMathLibrary.Vector_Up`))
  (bind _returnvalue_location (`KismetMathLibrary.BreakTransform` (`SceneComponent.GetRelativeTransform` (`self.Galaxy`))))
  (`SceneComponent.K2_SetRelativeRotation` (`self.Galaxy`) (`KismetMathLibrary.ComposeRotators` (`KismetMathLibrary.NegateRotator` (`KismetMathLibrary.MakeRotFromXZ` (.location (`.LocalGrabPoint` (break `UxtGrabPointerData` GrabPointer))) _returnvalue)) (`KismetMathLibrary.MakeRotFromXZ` (- (`KismetMathLibrary.InverseTransformLocation` (`self.GetParentTransform` null) (`UxtGrabPointerDataFunctionLibrary.GetTargetLocation` GrabPointer)) _returnvalue_location) _returnvalue)) false false))

(fn `UserConstructionScript`)