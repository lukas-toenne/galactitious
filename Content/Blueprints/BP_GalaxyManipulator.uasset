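; BP_GalaxyManipulator is a grabbable actor that gives material-based visual feedback when focused or grabbed.
; At BeginPlay it creates a dynamic instance of MI_Grabbable on its Mesh.
; Events from its BP_GalaxyGrabTarget drive two helper functions that set the material's focus and grab parameters.
; Grab begin, update and end also pass the grab location, computed from the actor transform and pointer data, into the material.
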(event `self.ReceiveBeginPlay`
  (bind _returnvalue (`PrimitiveComponent.CreateDynamicMaterialInstance` (`self.Mesh`) 0 "/Game/Materials/MI_Grabbable.MI_Grabbable" "None"))
  (set `self.Material` _returnvalue))

(event `self.BP_GalaxyGrabTarget.OnBeginGrab`
  (params (Grabbable :type "UxtGrabTargetComponent Object Reference") (GrabPointer :type "UxtGrabPointerData Structure"))
  (`self.UpdateMaterialGrab` true GrabPointer))

(event `self.BP_GalaxyGrabTarget.OnEnterFocus`
  (params (Pointer :type "UxtNearPointerComponent Object Reference"))
  (`self.UpdateMaterialFocus` true))

(event `self.BP_GalaxyGrabTarget.OnUpdateGrab`
  (params (Grabbable :type "UxtGrabTargetComponent Object Reference") (GrabPointer :type "UxtGrabPointerData Structure"))
  (`self.UpdateMaterialGrab` true GrabPointer))

(event `self.BP_GalaxyGrabTarget.OnUpdateFocus`
  (params (Pointer :type "UxtNearPointerComponent Object Reference")))

(event `self.BP_GalaxyGrabTarget.OnEndGrab`
  (params (Grabbable :type "UxtGrabTargetComponent Object Reference") (GrabPointer :type "UxtGrabPointerData Structure"))
  (`self.UpdateMaterialGrab` false GrabPointer))

(event `self.BP_GalaxyGrabTarget.OnExitFocus`
  (params (Pointer :type "UxtNearPointerComponent Object Reference"))
  (`self.UpdateMaterialFocus` false))

(fn `UpdateMaterialFocus`
  (params (IsFocused :type Boolean))
  (`MaterialInstanceDynamic.SetScalarParameterValue` (`self.Material`) "IsFocused" (`KismetMathLibrary.Conv_BoolToDouble` IsFocused)))

(fn `UpdateMaterialGrab`
  (params (IsGrabbed :type Boolean) (GrabPointerData :type "UxtGrabPointerData Structure (by ref)"))
  (bind _material (`self.Material`))
  (`MaterialInstanceDynamic.SetScalarParameterValue` _material "IsGrabbed" (`KismetMathLibrary.Conv_BoolToDouble` IsGrabbed))
  (`MaterialInstanceDynamic.SetVectorParameterValue` _material "GrabPosition" (`KismetMathLibrary.Conv_VectorToLinearColor` (`UxtGrabPointerDataFunctionLibrary.GetGrabLocation` (`self.GetTransform`) GrabPointerData))))

(fn `UserConstructionScript`)