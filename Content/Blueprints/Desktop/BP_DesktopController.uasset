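; BP_DesktopController is a player controller for desktop play that shows an on-screen UI widget to the local player.
; On BeginPlay it creates the configured widget class, adds it to the viewport, shows the mouse cursor and sets Game and UI input focused on the widget.
; On EndPlay it removes the widget and restores game-only input, with both steps limited to the local controller.
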(event `self.ReceiveBeginPlay`
  (`parent.ReceiveBeginPlay`)
  (if (`self.IsLocalPlayerController`)
    (`self.EnableUI`)))

(event `self.ReceiveEndPlay`
  (params (EndPlayReason :type "EEndPlayReason Enum" :default "Destroyed"))
  (`parent.ReceiveEndPlay` EndPlayReason)
  (if (`self.IsLocalPlayerController`)
    (`self.DisableUI`)))

(fn `DisableUI`
  (`Widget.RemoveFromParent` (`self.Widget`))
  (`WidgetBlueprintLibrary.SetInputMode_GameOnly` self))

(fn `EnableUI`
  (bind _returnvalue (`|CreateWidget` (`self.WidgetClass`) self))
  (bind _output_get (set `self.Widget` _returnvalue))
  (`UserWidget.AddToViewport` _output_get 0)
  (`WidgetBlueprintLibrary.SetInputMode_GameAndUIEx` self _output_get "DoNotLock" false)
  (set `self.bShowMouseCursor` true))

(fn `UserConstructionScript`)