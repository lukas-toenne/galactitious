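; BP_DesktopPawn is a desktop pawn with look, turn and zoom camera controls.
; LookUp and Turn axis inputs feed controller pitch and yaw, while Zoom calls AddCameraZoom.
; AddCameraZoom scales the camera's negative relative X offset exponentially by the axis value, so steps are proportional to distance, and clamps it between the minimum and maximum zoom distances.
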(event `InputAxis|LookUp`
  (params (AxisValue :type "Float (single-precision)"))
  (`self.AddControllerPitchInput` AxisValue))

(event `InputAxis|Turn`
  (params (AxisValue :type "Float (single-precision)"))
  (`self.AddControllerYawInput` AxisValue))

(event `InputAxis|Zoom`
  (params (AxisValue :type "Float (single-precision)"))
  (`self.AddCameraZoom` AxisValue))

(fn `AddCameraZoom`
  (params (AxisValue :type "Float (double-precision)"))
  (bind _camera (`self.Camera`))
  (bind _relativelocation_x (`KismetMathLibrary.BreakVector` (`SceneComponent.RelativeLocation` _camera)))
  (`SceneComponent.K2_SetRelativeLocation` _camera (`KismetMathLibrary.MakeVector` (`KismetMathLibrary.FClamp` (* _relativelocation_x (`KismetMathLibrary.Exp` (- 0.0 AxisValue))) (- 0.0 (`self.MaxZoom`)) (- 0.0 (`self.MinZoom`)))) false false))

(fn `UserConstructionScript`)