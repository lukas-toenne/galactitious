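; BP_GalaxySimulationActor displays a galaxy simulation by feeding its particle positions into a Niagara system.
; It binds to the Simulation's reset and step events and, on each, copies the position data into the Niagara "Positions" Float3 array data interface.
; Tick retries the upload and logs the result until one succeeds, then disables itself, leaving further updates to the simulation events.
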(event `self.ReceiveBeginPlay`
  (bind _simulation (`self.Simulation`))
  (add `FastMultipoleSimulation.OnSimulationReset` _simulation (delegate `OnSimulationReset`))
  (add `FastMultipoleSimulation.OnSimulationStep` _simulation (delegate `OnSimulationStep`)))

(event `OnSimulationReset`
  (params (Simulation :type "FastMultipoleSimulation Object Reference"))
  (`self.UploadNiagaraPointData` :!label _label))

(event `OnSimulationStep`
  (params (Simulation :type "FastMultipoleSimulation Object Reference"))
  (goto _label))

(event `self.ReceiveTick`
  (params (DeltaSeconds :type "Float (single-precision)"))
  (bind _success (`self.UploadNiagaraPointData`))
  (if _success
    (`KismetSystemLibrary.PrintString` "Niagara initialized!")
    (`self.SetActorTickEnabled` false)
    (else
      (`KismetSystemLibrary.PrintString` "Niagara upload failed"))))

(fn `UploadNiagaraPointData`
  (returns (Success :type Boolean))
  (bind _returnvalue (`NiagaraComponent.GetDataInterface` (`self.Niagara`) "Positions"))
  (`/Engine/EditorBlueprintResources/StandardMacros.IsValid` null
    (:`Is Valid`
      (bind _asvector_array (cast `NiagaraDataInterfaceArrayFloat3` _returnvalue)
        (:`then`
          (set `NiagaraDataInterfaceArrayFloat3.FloatData` (`FastMultipoleSimulation.GetPositionData` (`self.Simulation`)) _asvector_array)
          (return true))
        (:`CastFailed`
          (return false))))
    (:`Is Not Valid`
      (return false))))

(fn `UserConstructionScript`)