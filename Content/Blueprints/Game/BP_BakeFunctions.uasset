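; BP_BakeFunctions bakes textures into render targets: an inverse-CDF lookup from the RadialDensity curve, and a point spread function.
; BakeProbabilityCurve integrates, normalizes and inverts the density curve, converts it to a texture at the target's width, and draws it through a transient M_BakeTexture instance.
; BakeTextures runs that bake, then draws M_PointSpreadFunction directly to its own target.
; An optional debug flag draws the source, integrated and inverted curves as persistent lines.
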(fn `BakeProbabilityCurve`
  (params (CurveAsset :type "CurveFloat Object Reference") (TextureRenderTarget :type "TextureRenderTarget2D Object Reference") (DrawDebug :type Boolean))
  (locals (DebugTransform :type "Transform Structure" :default "0.000000,0.000000,0.000000|0.000000,0.000000,0.000000|100.000000,100.000000,100.000000") (BaseSettings :type "DrawDebugCurveSettings Structure") (IntegrateSettings :type "DrawDebugCurveSettings Structure") (InvertSettings :type "DrawDebugCurveSettings Structure"))
  (`|ExecutionSequence`
    (:`then_0`
      (bind _curve (`ProbabilityCurveFunctionLibrary.ConvertCurveAsset` CurveAsset))
      (bind _integratedcurve (`ProbabilityCurveFunctionLibrary.IntegrateCurve` _curve))
      (bind _normalizedcurve (`ProbabilityCurveFunctionLibrary.NormalizeCurve` _integratedcurve))
      (bind _invertedcurve (`ProbabilityCurveFunctionLibrary.InvertCurve` _normalizedcurve 10))
      (bind _returnvalue (`ProbabilityCurveFunctionLibrary.CurveToTexture2D` _invertedcurve (`TextureRenderTarget2D.SizeX` TextureRenderTarget)))
      (bind _returnvalue_2 (`KismetMaterialLibrary.CreateDynamicMaterialInstance` (`local.__WorldContext`) "/Game/Materials/M_BakeTexture.M_BakeTexture" "None" "Transient"))
      (`MaterialInstanceDynamic.SetTextureParameterValue` _returnvalue_2 "Tex" _returnvalue)
      (`KismetRenderingLibrary.DrawMaterialToRenderTarget` (`local.__WorldContext`) TextureRenderTarget _returnvalue_2))
    (:`then_1`
      (if DrawDebug
        (`ProbabilityCurveFunctionLibrary.DrawDebugCurve` (`local.__WorldContext`) _curve (`local.DebugTransform`) (`local.BaseSettings`) true)
        (`ProbabilityCurveFunctionLibrary.DrawDebugCurve` (`local.__WorldContext`) _integratedcurve (`local.DebugTransform`) (`local.IntegrateSettings`) true)
        (`ProbabilityCurveFunctionLibrary.DrawDebugCurve` (`local.__WorldContext`) _invertedcurve (`local.DebugTransform`) (`local.InvertSettings`) true)))))

(fn `BakeTextures`
  (params (DrawDebug :type Boolean))
  (bind ___worldcontext (`local.__WorldContext`))
  (`self.BakeProbabilityCurve` "/Game/Curves/RadialDensity.RadialDensity" "/Game/Textures/T_RadialDensity.T_RadialDensity" ___worldcontext DrawDebug)
  (`KismetRenderingLibrary.DrawMaterialToRenderTarget` ___worldcontext "/Game/Textures/T_PointSpreadFunction.T_PointSpreadFunction" "/Game/Materials/M_PointSpreadFunction.M_PointSpreadFunction"))