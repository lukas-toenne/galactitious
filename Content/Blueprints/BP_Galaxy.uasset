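; BP_Galaxy is an actor that feeds a radial density distribution into a Niagara particle system, apparently to shape a galaxy.
; On BeginPlay it converts the RadialDensity curve, then integrates, normalizes and inverts it, building an inverse CDF for inverse transform sampling.
; The result is baked into a small texture and passed to the Particles system as TestTex.
; A disconnected construction-script chain holds debug drawing of the curve stages.
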(event `self.ReceiveBeginPlay`
  (bind _curve (`ProbabilityCurveFunctionLibrary.ConvertCurveAsset` "/Game/Curves/RadialDensity.RadialDensity"))
  (bind _integratedcurve (`ProbabilityCurveFunctionLibrary.IntegrateCurve` _curve))
  (bind _normalizedcurve (`ProbabilityCurveFunctionLibrary.NormalizeCurve` _integratedcurve))
  (bind _invertedcurve (`ProbabilityCurveFunctionLibrary.InvertCurve` _normalizedcurve))
  (bind _returnvalue (`ProbabilityCurveFunctionLibrary.CurveToTexture2D` _invertedcurve 53))
  (`NiagaraFunctionLibrary.SetTextureObject` (`self.Particles`) "TestTex" _returnvalue))

(fn `UserConstructionScript`
  (locals (DrawDebugTransform :type "Transform Structure" :default "0.000000,0.000000,0.000000|0.000000,0.000000,0.000000|100.000000,100.000000,100.000000") (DrawCurveSettings_Original :type "DrawDebugCurveSettings Structure" :default (struct :`CurveResolution` 30 :`PointSize` 3.0 :`PointColor` (struct :`B` 255 :`G` 255 :`R` 255 :`A` 255) :`LineColor` (struct :`B` 170 :`G` 147 :`R` 64 :`A` 255) :`TangentColor` (struct :`G` 255 :`R` 255 :`A` 255))) (DrawCurveSettings_Integrated :type "DrawDebugCurveSettings Structure" :default (struct :`CurveResolution` 30 :`PointSize` 3.0 :`PointColor` (struct :`B` 255 :`G` 255 :`R` 255 :`A` 255) :`LineColor` (struct :`B` 230 :`G` 77 :`R` 233 :`A` 255) :`TangentColor` (struct :`G` 255 :`R` 255 :`A` 255))) (DrawCurveSettings_Inverted :type "DrawDebugCurveSettings Structure" :default (struct :`CurveResolution` 30 :`PointSize` 3.0 :`PointColor` (struct :`B` 255 :`G` 255 :`R` 255 :`A` 255) :`LineColor` (struct :`B` 53 :`G` 178 :`R` 102 :`A` 255) :`TangentColor` (struct :`G` 255 :`R` 255 :`A` 255)))))