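; BP_GalaxyRimManipulator builds a ring of capsule collision components, apparently as the rim handle of a galaxy.
; The construction script adds one capsule per segment, laid tangentially at the edge midpoints of a regular polygon inscribed in Radius.
; Capsule half-height is half the chord plus half Thickness, so rounded caps meet at the polygon's corners.
; BeginPlay only calls the parent, and the UI collision profile and overlap-disabling nodes are unconnected.
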(event `self.ReceiveBeginPlay`
  (`parent.ReceiveBeginPlay`))

(event `self.ReceiveTick`
  (params (DeltaSeconds :type "Float (single-precision)")))

(fn `UserConstructionScript`
  (bind _segments (`self.Segments`))
  (bind _radius (`self.Radius`))
  (bind _returnvalue (* (`self.Thickness`) 0.5))
  (bind _returnvalue_2 (/ 360.0 (`KismetMathLibrary.Conv_IntToDouble` _segments)))
  (bind _returnvalue_3 (* _returnvalue_2 0.5))
  (bind _returnvalue_4 (* _radius (`KismetMathLibrary.DegCos` _returnvalue_3)))
  (for _index (range _segments)
    (bind _returnvalue_5 (* _index _returnvalue_2))
    (bind _returnvalue_6 (`AddComponent|NODE_AddCapsuleComponent-0` :`RelativeTransform` (`KismetMathLibrary.MakeTransform` (`KismetMathLibrary.MakeVector` (* _returnvalue_4 (`KismetMathLibrary.DegCos` _returnvalue_5)) (* _returnvalue_4 (`KismetMathLibrary.DegSin` _returnvalue_5))) (`KismetMathLibrary.MakeRotator` 90.0 0.0 _returnvalue_5))))
    (`CapsuleComponent.SetCapsuleSize` _returnvalue_6 _returnvalue (+ _returnvalue (* _radius (`KismetMathLibrary.DegSin` _returnvalue_3))) false)))